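; Spawner that drops an instance of its Ingredient class when SpawnIngredient fires while the player pawn overlaps its Trigger.
; It sends a SpawnIngredientMessage to Target, then spawns at a random point in a box around the Mesh, raised by SpawnHeight.
; Each spawn gets random roll and yaw, a slight random pitch and a random uniform scale, and the Trigger component moves slightly down.
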(event `/Game/ThirdPerson/Blueprints/BPI_Interact.SpawnIngredient`
  (bind (_returnvalue_roll _returnvalue_pitch _returnvalue_yaw) (`KismetMathLibrary.BreakRotator` (`KismetMathLibrary.RandomRotator` false)))
  (bind _trigger (`self.Trigger`))
  (bind (_relativelocation_x _relativelocation_y _relativelocation_z) (`KismetMathLibrary.BreakVector` (`SceneComponent.RelativeLocation` _trigger)))
  (bind (_returnvalue_x _returnvalue_y _returnvalue_z) (`KismetMathLibrary.BreakVector` (`KismetMathLibrary.RandomPointInBoundingBox` (`SceneComponent.K2_GetComponentLocation` (`self.Mesh`)) (200.0 200.0 40.0))))
  (if (`PrimitiveComponent.IsOverlappingActor` (`self.Trigger`) (`GameplayStatics.GetPlayerPawn` 0))
    (message `/Game/ThirdPerson/Blueprints/BPI_Interact.SpawnIngredient` (`self.Target`))
    (`|ExecutionSequence`
      (:`then_0`
        (`|SpawnActorFromClass` (`self.Ingredient`) (`KismetMathLibrary.MakeTransform` (`KismetMathLibrary.MakeVector` _returnvalue_x _returnvalue_y (+ _returnvalue_z (`self.SpawnHeight`))) (`KismetMathLibrary.MakeRotator` _returnvalue_roll (`KismetMathLibrary.RandomFloatInRange` 0.0 15.0) _returnvalue_yaw) (`KismetMathLibrary.Conv_DoubleToVector` (`KismetMathLibrary.RandomFloatInRange` (`self.MinScale`) (`self.MaxScale`)))) "Undefined" "OverrideRootScale" null null))
      (:`then_1`
        (`KismetSystemLibrary.MoveComponentTo` _trigger (`KismetMathLibrary.MakeVector` _relativelocation_x _relativelocation_y (- _relativelocation_z 5.0)))))))

(fn `UserConstructionScript`)