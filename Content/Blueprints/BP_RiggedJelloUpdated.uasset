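; Rigged jello actor that serves as a configurable skeletal mesh prop with selectable look and shape.
; The construction script uses ID variables to pick the material, skeletal mesh and matching physics asset from arrays.
; BeginPlay and the mesh hit event are empty.
; Disconnected, never-run chains hold character-triggered logic for toggling physics simulation and briefly disabling collision when the third-person character jumps.
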(event `self.ReceiveBeginPlay`)

(event `self.SkeletalMesh.OnComponentHit`
  (params (HitComponent :type "PrimitiveComponent Object Reference") (OtherActor :type "Actor Object Reference") (OtherComp :type "PrimitiveComponent Object Reference") (NormalImpulse :type "Vector Structure") (Hit :type "HitResult Structure (by ref)")))

(fn `UserConstructionScript`
  (`|ExecutionSequence`
    (:`then_0`
      ;[1 1 1] Change the material instance
      (`PrimitiveComponent.SetMaterial` (`self.SkeletalMesh`) 0 (`|GetArrayItem` (`self.Materials`) (`self.MaterialID`))))
    (:`then_1`
      ;[1 1 1] Change the mesh
      (`SkeletalMeshComponent.SetSkeletalMeshAsset` (`self.SkeletalMesh`) (`|GetArrayItem` (`self.Meshes`) (`self.MeshID`))))
    (:`then_2`
      ;[1 1 1] Change physics asset to match the new mesh
      (`SkinnedMeshComponent.SetPhysicsAsset` (`self.SkeletalMesh`) (`|GetArrayItem` (`self.PhysicsAsset`) (`self.PhysicsAssetID`)) false))))