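; BP_Goo is a physics-simulated goo ball pickup that the third-person character collects by touching it.
; On the first overlap with BP_ThirdPersonCharacter, it sets a one-shot picked flag, triggers the character's pickup behavior and increments its goo total.
; The ball then stops simulating physics and destroys itself after a short delay.
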(event `self.ReceiveBeginPlay`
  (`PrimitiveComponent.SetSimulatePhysics` (`self.GooBall`) true))

(event `self.GooBall.OnComponentBeginOverlap`
  (params (OverlappedComponent :type "PrimitiveComponent Object Reference") (OtherActor :type "Actor Object Reference") (OtherComp :type "PrimitiveComponent Object Reference") (OtherBodyIndex :type Integer) (bFromSweep :type Boolean) (SweepResult :type "HitResult Structure (by ref)"))
  (if (not (`self.IsPicked?`))
    (bind _asbp_third_person_character (cast `/Game/ThirdPerson/Blueprints/BP_ThirdPersonCharacter` OtherActor))
    (set `self.IsPicked?` true)
    (set `/Game/ThirdPerson/Blueprints/BP_ThirdPersonCharacter.IsPickingUp?` true _asbp_third_person_character)
    (`/Game/ThirdPerson/Blueprints/BP_ThirdPersonCharacter.PickingUp` _asbp_third_person_character)
    (`/Engine/EditorBlueprintResources/StandardMacros.IncrementInt` (`/Game/ThirdPerson/Blueprints/BP_ThirdPersonCharacter.TotalGooAmt` _asbp_third_person_character)
      (:`  `
        (`PrimitiveComponent.SetSimulatePhysics` (`self.GooBall`) false)
        (`KismetSystemLibrary.Delay` 0.5)
        (`self.K2_DestroyActor`)))))

(fn `UserConstructionScript`)