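; BP_Projectile is a short-lived projectile actor that can act as a collectible water droplet.
; On BeginPlay it caches the player character, enables physics on its collision sphere after a brief delay, then destroys itself shortly afterward.
; Any sphere overlap stores the other actor, sends it the droplet amount through a WaterCountMessage call if flagged as a water droplet, and destroys the projectile.
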(event `self.ReceiveBeginPlay`
  ;[0 1 0] Init
  (bind _asbp_third_person_character (cast `/Game/ThirdPerson/Blueprints/BP_ThirdPersonCharacter` (`GameplayStatics.GetPlayerPawn` 0)))
  (set `self.TP Char Ref` _asbp_third_person_character)
  (`KismetSystemLibrary.Delay` 0.2)
  (`PrimitiveComponent.SetSimulatePhysics` (`self.SphereCollision`) true)
  (`KismetSystemLibrary.Delay` 1.6)
  (`self.K2_DestroyActor`))

(event `CollectWater`
  ;[0.1757 0 0.6198] Collect water droplet
  (if (`self.IsWaterDroplet?`)
    (message `/Game/ThirdPerson/Blueprints/BPI_Player.WaterCount` (`self.Other Actor`) (`self.WaterDropletAmt`))
    (`KismetSystemLibrary.PrintString` "+1 water droplet")))

(event `self.SphereCollision.OnComponentBeginOverlap`
  (params (OverlappedComponent :type "PrimitiveComponent Object Reference") (OtherActor :type "Actor Object Reference") (OtherComp :type "PrimitiveComponent Object Reference") (OtherBodyIndex :type Integer) (bFromSweep :type Boolean) (SweepResult :type "HitResult Structure (by ref)"))
  ;[0.1757 0 0.6198] Collect water droplet
  (set `self.Other Actor` OtherActor)
  (`|ExecutionSequence`
    (:`then_0`
      (`self.CollectWater`)
      (`self.K2_DestroyActor`))))

(fn `UserConstructionScript`)