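; BP_Respawn replaces actors from its Spawns list once they are no longer valid.
; At BeginPlay it records their transforms in a parallel array and starts a looping timer with an interval randomized once between fixed bounds.
; Each check spawns SpawnClass at an invalid entry's saved transform, moving that slot to the end of both arrays while still iterating over Spawns.
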(event `self.ReceiveBeginPlay`
  (for _array_element (`self.Spawns`)
    (`KismetArrayLibrary.Array_Add` (`self.SpawnTransforms`) (`self.GetTransform` _array_element)))
  (`KismetSystemLibrary.K2_SetTimerDelegate` (delegate `CheckSpawns`) (`KismetMathLibrary.RandomFloatInRange` 10.0 20.0) true))

(event `CheckSpawns`
  (bind _spawns (`self.Spawns`))
  (for (_array_element _array_index) _spawns
    (`/Engine/EditorBlueprintResources/StandardMacros.IsValid` _array_element
      (:`Is Not Valid`
        (`KismetArrayLibrary.Array_Remove` _spawns _array_index)
        (bind _returnvalue (`|SpawnActorFromClass` (`self.SpawnClass`) (`|GetArrayItem` (`self.SpawnTransforms`) _array_index) "Undefined" "OverrideRootScale" null null))
        (`KismetArrayLibrary.Array_Remove` (`self.SpawnTransforms`) _array_index)
        (`KismetArrayLibrary.Array_Add` (`self.SpawnTransforms`) (`self.GetTransform` _returnvalue))
        (`KismetArrayLibrary.Array_Add` (`self.Spawns`) _returnvalue)))))

(fn `UserConstructionScript`)