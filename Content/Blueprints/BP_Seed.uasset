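; BP_Seed is a seed actor that grows into a cherry tree and then produces a jello actor.
; GrowSeed runs a timed sequence of delays that scales up the Seed mesh, swaps it to the cherry tree mesh, then spawns a BP_RiggedJelloUpdated at an offset above it.
; The construction script sets the seed's material from a Materials array using MaterialID.
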(event `GrowSeed`
  (bind _seed (`self.Seed`))
  (`KismetSystemLibrary.Delay` 5.0)
  (`SceneComponent.SetWorldScale3D` _seed (3.0 3.0 3.0))
  (`KismetSystemLibrary.Delay` 5.0)
  (`StaticMeshComponent.SetStaticMesh` _seed "/Game/InfinityBladeGrassLands/Environments/Earth/StaticMesh/SM_Cherry_Tree.SM_Cherry_Tree")
  (`KismetSystemLibrary.Delay` 5.0)
  (`|SpawnActorFromClass` "/Game/Blueprints/BP_RiggedJelloUpdated.BP_RiggedJelloUpdated_C" (`KismetMathLibrary.MakeTransform` (+ (`SceneComponent.K2_GetComponentLocation` _seed) (180.0 180.0 500.0))) "Undefined" "OverrideRootScale" null null))

(fn `UserConstructionScript`
  ;[1 1 1] Change the material instance
  (`PrimitiveComponent.SetMaterial` (`self.Seed`) 0 (`|GetArrayItem` (`self.Materials`) (`self.Material ID`))))