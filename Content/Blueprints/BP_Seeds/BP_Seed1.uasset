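; Seed actor that grows in timed stages, then spawns jello pickups, with a random material set on construction.
; GrowSeed uses delays to step through scales and a mesh swap with random yaw, then runs a looping SpawnPickups timer for a limited window.
; Each BP_RiggedJelloUpdated gets random scale, mesh and material.
; Its physics asset is indexed by appending another random mesh to Meshes, so it is not matched to the displayed mesh.
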(event `GrowSeed`
  (bind (_returnvalue_roll _returnvalue_pitch _returnvalue_yaw) (`KismetMathLibrary.BreakRotator` (`KismetMathLibrary.RandomRotator` false)))
  (bind _seed (`self.Seed`))
  (bind _seed_2 (`self.Seed`))
  (`KismetSystemLibrary.Delay` 5.0)
  (`SceneComponent.SetWorldScale3D` _seed (`self.New Scale 1`))
  (`KismetSystemLibrary.Delay` 5.0)
  (`StaticMeshComponent.SetStaticMesh` _seed (`self.New Mesh`))
  (`SceneComponent.K2_SetWorldTransform` _seed_2 (`KismetMathLibrary.MakeTransform` (`SceneComponent.K2_GetComponentLocation` _seed_2) (`KismetMathLibrary.MakeRotator` 0.0 0.0 _returnvalue_yaw)) false false)
  (`SceneComponent.SetWorldScale3D` (`self.Seed`) (`self.New Scale 2`))
  (`KismetSystemLibrary.Delay` 5.0)
  (`SceneComponent.SetWorldScale3D` (`self.Seed`) (`self.New Scale 3`))
  (`KismetSystemLibrary.Delay` 5.0)
  (bind _returnvalue (`KismetSystemLibrary.K2_SetTimerDelegate` (delegate `SpawnPickups`) 5.0 true))
  (`KismetSystemLibrary.Delay` 20.0)
  (`KismetSystemLibrary.K2_PauseTimerHandle` _returnvalue))

(event `SpawnPickups`
  (bind _returnvalue (`|SpawnActorFromClass` "/Game/Blueprints/BP_RiggedJelloUpdated.BP_RiggedJelloUpdated_C" (`KismetMathLibrary.MakeTransform` (+ (`SceneComponent.K2_GetComponentLocation` (`self.Seed`)) (`self.NewSpawnLocation`)) (`KismetMathLibrary.MakeRotator` 0.0) (`KismetMathLibrary.Conv_DoubleToVector` (`KismetMathLibrary.RandomFloatInRange` 0.3 2.3))) "Undefined" "OverrideRootScale" null null))
  (bind _skeletalmesh (`/Game/Blueprints/BP_RiggedJelloUpdated.SkeletalMesh` _returnvalue))
  (bind _meshes (`/Game/Blueprints/BP_RiggedJelloUpdated.Meshes` _returnvalue))
  (bind _outitem (`KismetArrayLibrary.Array_Random` _meshes))
  (`SkeletalMeshComponent.SetSkeletalMeshAsset` _skeletalmesh _outitem)
  (bind _returnvalue_2 (`KismetArrayLibrary.Array_Add` _meshes _outitem))
  (`SkinnedMeshComponent.SetPhysicsAsset` _skeletalmesh (`|GetArrayItem` (`/Game/Blueprints/BP_RiggedJelloUpdated.PhysicsAsset` _returnvalue) _returnvalue_2) false)
  (`PrimitiveComponent.SetMaterial` _skeletalmesh 0 (`KismetArrayLibrary.Array_Random` (`/Game/Blueprints/BP_RiggedJelloUpdated.Materials` _returnvalue)))
  (`PrimitiveComponent.SetConstraintMode` _skeletalmesh "None"))

(fn `UserConstructionScript`
  ;[1 1 1] Change the material instance
  (`PrimitiveComponent.SetMaterialByName` (`self.Seed`) "red" (`|GetArrayItem` (`self.Materials`) (`KismetMathLibrary.RandomIntegerInRange` 0 5))))